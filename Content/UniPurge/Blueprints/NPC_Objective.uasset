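; NPC objective pawn that navigates to destinations and flees when it detects the player (Jugador), gated by an Active flag.
; EmpezarNavegar runs AIMoveTo and calls PointReached on success or failure.
; Tick checks two overlap senses: View triggers escape toward a macro-supplied point, otherwise SoundHearer slowly turns it toward the player.
; With neither overlapping, an ongoing escape ends through PointReached; the macro's negated-offset vector math is left unconnected.
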(event `self.EmpezarNavegar`
  (if (`self.active`)
    (`|AIMoveTo` self (`self.Destination`) null 40.0 true
      (:`OnSuccess`
        _)
      (:`OnFail`
        _))
    (`self.PointReached` false)))

(event `self.ReceiveTick`
  (params (DeltaSeconds :type "Float (single-precision)"))
  (if (`self.active`)
    (if (`PrimitiveComponent.IsOverlappingActor` (`self.View`) (`.jugador` (`self.jugador`)))
      (set `self.Escapando` true)
      (`|AIMoveTo` self (`self.NewMacro_0`) null 40.0 true)
      (elif (`PrimitiveComponent.IsOverlappingActor` (`self.Sound Hearer`) (`.jugador` (`self.jugador`)))
        (`self.K2_SetActorRotation` (`KismetMathLibrary.RInterpTo` (`self.K2_GetActorRotation` self) (`KismetMathLibrary.FindLookAtRotation` (`self.K2_GetActorLocation` self) (`self.K2_GetActorLocation` (`.jugador` (`self.jugador`)))) DeltaSeconds 1.0))
        (elif (`self.Escapando`)
          (set `self.Escapando` false)
          (`self.PointReached` false))))))

(fn `UserConstructionScript`)