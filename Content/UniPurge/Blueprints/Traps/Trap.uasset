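; Trap actor that loads its model on BeginPlay and controls an attached music cue.
; SettingShift stops the audio when passed true; when false, it spawns the cue on the static mesh or replays the existing component.
; Replays start at a random offset bounded by MaxTime within a 120-second window, while the first spawn starts from the beginning.
; Destroying the trap stops the sound.
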(event `self.ReceiveDestroyed`
  (bind _sound (`self.Sound`))
  (if (`KismetSystemLibrary.IsValid` _sound)
    (`AudioComponent.Stop` _sound)))

(event `self.SettingShift`
  (params (onOrOff :type Boolean))
  (bind _sound (`self.Sound`))
  (bind _returnvalue (`KismetSystemLibrary.IsValid` _sound))
  (if onOrOff
    (if _returnvalue
      (`AudioComponent.Stop` _sound))
    (elif _returnvalue
      (`AudioComponent.Play` (`self.Sound`) (`KismetMathLibrary.RandomFloatInRange` 0.0 (- 120.0 (`self.MaxTime`))))
      (else
        (bind _returnvalue_2 (`GameplayStatics.SpawnSoundAttached` "/Game/UniPurge/Sounds/Mr_Smith_-_Remember_Cue.Mr_Smith_-_Remember_Cue" (`self.StaticMesh`) "None" (0.0 0.0 0.0) (struct) "KeepRelativeOffset" false 1.0 1.0 0.0 null null))
        (set `self.Sound` _returnvalue_2)))))

(event `self.ReceiveBeginPlay`
  (`self.LoadModel`))

(fn `UserConstructionScript`)